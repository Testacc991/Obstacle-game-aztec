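; MyChar is a player Character Blueprint with basic movement, look and jump controls.
; Axis inputs turn controller yaw and pitch and add movement along the capsule's forward and right vectors, while a jump action calls Jump.
; When destroyed, it casts the game mode to MyGameMode and asks it to respawn using SpawnCoordinates.
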(event EventDestroyed
  (bind _asmy_game_mode (Utilities|Casting|CastToMyGameMode (Game|GetGameMode)))
  (Default|Respawn _asmy_game_mode (Variables|Default|GetSpawnCoordinates)))

(event Input|ActionEvents|InputActionJumpCustom1
  (params (Key :type Key%20Structure :default "None"))
  (:Pressed
    (Character|Jump)))

(event Input|AxisEvents|InputAxisLookUP
  (params (AxisValue :type Float%20%28single-precision%29))
  (Pawn|Input|AddControllerPitchInput AxisValue))

(event Input|AxisEvents|InputAxisLookLR
  (params (AxisValue :type Float%20%28single-precision%29))
  (Pawn|Input|AddControllerYawInput AxisValue))

(event Input|AxisEvents|InputAxisMoveFB
  (params (AxisValue :type Float%20%28single-precision%29))
  (Pawn|Input|AddMovementInput (Math|Vector|GetForwardVector (Variables|Collision|GetCapsuleComponent)) AxisValue false))

(event Input|AxisEvents|InputAxisMoveLR
  (params (AxisValue :type Float%20%28single-precision%29))
  (Pawn|Input|AddMovementInput (Math|Vector|GetRightVector (Variables|Collision|GetCapsuleComponent)) AxisValue false))

(fn ConstructionScript)