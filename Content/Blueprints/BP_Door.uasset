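; BP_Door is a two-panel sliding door actor that opens and closes as things enter or leave its trigger boxes.
; Each side is independent: overlapping Boxleft or Boxright plays that side's timeline, which drives the panel's relative location, and ending the overlap reverses it.
; Every begin and end overlap plays an attenuated door-moving sound at the actor's location, with no filter on the overlapping actor.
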(event OnComponentEndOverlap(Boxleft)
  (params (OverlappedComponent :type Primitive%20Component%20Object%20Reference) (OtherActor :type Actor%20Object%20Reference) (OtherComp :type Primitive%20Component%20Object%20Reference) (OtherBodyIndex :type Integer))
  (Audio|PlaySoundatLocation "/Game/Sounds/doormoving.doormoving" (Transformation|GetActorLocation) "0, 0, 0" 1.0 1.0 0.0 "/Game/Sounds/doormovesound.doormovesound" 0 0 0)
  (bind _newtrack_0 (Timeline|lefttimeline Reverse)
    (:Update
      (Transformation|SetRelativeLocation (Variables|Default|Getdoorleft) _newtrack_0 false false))))

(event OnComponentBeginOverlap(Boxleft)
  (params (OverlappedComponent :type Primitive%20Component%20Object%20Reference) (OtherActor :type Actor%20Object%20Reference) (OtherComp :type Primitive%20Component%20Object%20Reference) (OtherBodyIndex :type Integer) (bFromSweep :type Boolean) (SweepResult :type Hit%20Result%20Structure%20%28by%20ref%29))
  (Audio|PlaySoundatLocation "/Game/Sounds/doormoving.doormoving" (Transformation|GetActorLocation) "0, 0, 0" 1.0 1.0 0.0 "/Game/Sounds/doormovesound.doormovesound" 0 0 0)
  (bind _newtrack_0 (Timeline|lefttimeline Play)
    (:Update
      (Transformation|SetRelativeLocation (Variables|Default|Getdoorleft) _newtrack_0 false false))))

(event OnComponentBeginOverlap(Boxright)
  (params (OverlappedComponent :type Primitive%20Component%20Object%20Reference) (OtherActor :type Actor%20Object%20Reference) (OtherComp :type Primitive%20Component%20Object%20Reference) (OtherBodyIndex :type Integer) (bFromSweep :type Boolean) (SweepResult :type Hit%20Result%20Structure%20%28by%20ref%29))
  (Audio|PlaySoundatLocation "/Game/Sounds/doormoving.doormoving" (Transformation|GetActorLocation) "0, 0, 0" 1.0 1.0 0.0 "/Game/Sounds/doormovesound.doormovesound" 0 0 0)
  (bind _newtrack_0 (Timeline|Righttimeline Play)
    (:Update
      (Transformation|SetRelativeLocation (Variables|Default|Getdoorright) _newtrack_0 false false))))

(event OnComponentEndOverlap(Boxright)
  (params (OverlappedComponent :type Primitive%20Component%20Object%20Reference) (OtherActor :type Actor%20Object%20Reference) (OtherComp :type Primitive%20Component%20Object%20Reference) (OtherBodyIndex :type Integer))
  (Audio|PlaySoundatLocation "/Game/Sounds/doormoving.doormoving" (Transformation|GetActorLocation) "0, 0, 0" 1.0 1.0 0.0 "/Game/Sounds/doormovesound.doormovesound" 0 0 0)
  (bind _newtrack_0 (Timeline|Righttimeline Reverse)
    (:Update
      (Transformation|SetRelativeLocation (Variables|Default|Getdoorright) _newtrack_0 false false))))

(fn ConstructionScript)