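; BP_Cylinder2 is an actor with a cylinder component that spins continuously around its yaw axis while two audio components play.
; BeginPlay starts both audio components from the beginning.
; Tick adds delta time plus a fixed step to a rotation value, making the speed frame-rate dependent, and applies it as relative yaw.
; The value resets to zero after a full turn.
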(event EventBeginPlay
  (Utilities|FlowControl|Sequence
    (:then_0
      (Audio|Components|Audio|Play (Variables|Default|GetAudio) 0.0))
    (:then_1
      (Audio|Components|Audio|Play (Variables|Default|GetAudio1) 0.0))))

(event Collision|EventActorBeginOverlap
  (params (OtherActor :type Actor%20Object%20Reference)))

(event EventTick
  (params (DeltaSeconds :type Float%20%28single-precision%29))
  (bind _output_get (Variables|Default|Setmult 1.5))
  (Variables|Default|SetRotation (+ DeltaSeconds (Variables|Default|GetRotation) _output_get))
  (if (< (Variables|Default|GetRotation) 3.6e+02)
    (Transformation|SetRelativeRotation (Variables|Default|Getcylynder) (Math|Rotator|MakeRotator 0.0 0.0 (Variables|Default|GetRotation)) false false)
    (else
      (Variables|Default|SetRotation 0.0))))

(fn ConstructionScript)