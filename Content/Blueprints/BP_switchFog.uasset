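; BP_switchFog is a trigger-box actor that clears height fog and hides the sky atmosphere while something overlaps its box.
; BeginPlay finds the ExponentialHeightFog and SkyAtmosphere actors by class and sets the default target density.
; Box begin and end overlap switch that target and toggle atmosphere visibility, without filtering the overlapping actor.
; Tick continuously interpolates fog density toward the target, so fog fades while the atmosphere switches instantly.
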(event OnComponentBeginOverlap(Box)
  (params (OverlappedComponent :type Primitive%20Component%20Object%20Reference) (OtherActor :type Actor%20Object%20Reference) (OtherComp :type Primitive%20Component%20Object%20Reference) (OtherBodyIndex :type Integer) (bFromSweep :type Boolean) (SweepResult :type Hit%20Result%20Structure%20%28by%20ref%29))
  (Variables|Default|SetFogDensityCustom 0.0)
  (Variables|Default|SetEnterExit false)
  (Rendering|SetVisibility (Variables|/Script/Engine.SkyAtmosphere|GetSkyAtmosphereComponent (stale EventBeginPlay _returnvalue_2)) (Variables|Default|GetEnterExit) false))

(event OnComponentEndOverlap(Box)
  (params (OverlappedComponent :type Primitive%20Component%20Object%20Reference) (OtherActor :type Actor%20Object%20Reference) (OtherComp :type Primitive%20Component%20Object%20Reference) (OtherBodyIndex :type Integer))
  (Variables|Default|SetFogDensityCustom 0.0436)
  (Variables|Default|SetEnterExit true)
  (Rendering|SetVisibility (Variables|/Script/Engine.SkyAtmosphere|GetSkyAtmosphereComponent (stale EventBeginPlay _returnvalue_2)) (Variables|Default|GetEnterExit) false))

(event EventBeginPlay
  (Variables|Default|SetFogDensityCustom 0.0436)
  (bind _returnvalue (Actor|GetActorOfClass "/Script/Engine.ExponentialHeightFog"))
  (bind _returnvalue_2 (Actor|GetActorOfClass "/Script/Engine.SkyAtmosphere")))

(event Collision|EventActorBeginOverlap
  (params (OtherActor :type Actor%20Object%20Reference)))

(event EventTick
  (params (DeltaSeconds :type Float%20%28single-precision%29))
  (Class|ExponentialHeightFogComponent|SetFogDensity (Variables|/Script/Engine.ExponentialHeightFog|GetComponent (stale EventBeginPlay _returnvalue)) (Math|Interpolation|FInterpTo (Variables|/Script/Engine.ExponentialHeightFogComponent|GetFogDensity (Variables|/Script/Engine.ExponentialHeightFog|GetComponent (stale EventBeginPlay _returnvalue))) (Variables|Default|GetFogDensityCustom) DeltaSeconds 1.0)))

(fn ConstructionScript)